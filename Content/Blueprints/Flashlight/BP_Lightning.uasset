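; BP_Lightning is a lightning effect actor that flickers a point light whenever its Flash event is called.
; Flash plays a timeline whose value, scaled through an arcsine and a random factor, randomly hides or shows the light on each update.
; Each update also randomizes the light's color temperature within a cool range and prints a debug value.
; When the timeline finishes, the light is left visible.
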(event `Flash`
  (bind _pointlight (`self.PointLight`))
  (bind (_direction _value) (`Timeline|Timeline` :!via `PlayFromStart`)
    (:`Update`
      (bind _returnvalue (* (`KismetMathLibrary.DegAsin` _value) (`KismetMathLibrary.RandomFloatInRange` -1.5 1.5)))
      (`KismetSystemLibrary.PrintString` (`KismetStringLibrary.Conv_DoubleToString` _returnvalue) true true (struct :`G` 0.66 :`B` 1.0 :`A` 1.0) _returnvalue)
      (`SceneComponent.SetHiddenInGame` _pointlight (> _returnvalue 0.0) false)
      (`LightComponent.SetTemperature` _pointlight (`KismetMathLibrary.RandomFloatInRange` 8292.0 12000.0)))
    (:`Finished`
      (`SceneComponent.SetHiddenInGame` _pointlight false false))))

(fn `UserConstructionScript`)